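; Control panel prop that toggles several linked objects at once when it receives a Pop interaction.
; The interaction event calls ActivateDeactivate on every entry in the BPActivatables array.
; After a short delay it spawns Niagara sparks at the Billboard's location, swaps one mesh material slot to BaseFlattenMaterial and plays a 2D panel sound.
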(event `/Game/Dynamic/Blueprints/Core/BPI_PopInteract.BPI_PopInteract`
  (for _array_element (`self.BP_Activatables`)
    (`/Game/Dynamic/Blueprints/Environment/Activatable/BP_ActivatableParent.Activate/Deactivate` _array_element))
  (`KismetSystemLibrary.Delay` 0.3)
  (`NiagaraFunctionLibrary.SpawnSystemAtLocation` "/Game/Dynamic/Blueprints/Environment/NS_Sparks.NS_Sparks" (`SceneComponent.K2_GetComponentLocation` (`self.Billboard`)))
  (`PrimitiveComponent.SetMaterial` (`self.StaticMesh`) 1 "/Engine/EngineMaterials/BaseFlattenMaterial.BaseFlattenMaterial")
  (`GameplayStatics.PlaySound2D` "/Game/Dynamic/Audio/Events/MS_ControlPanel.MS_ControlPanel" 1.0 1.0 0.0 null null))

(fn `UserConstructionScript`
  (`parent.UserConstructionScript`))